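; Player-controlled tank Blueprint that handles camera aim input and firing.
; On BeginPlay it passes the TankBarrel and TankTurret components to SetBarrelRef and SetTurretRef.
; AimX yaws the Gimbal and AimY pitches the SpringArm, separating the two rotation axes, while the Fire action calls Fire.
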(event `self.ReceiveBeginPlay`
  (`self.SetBarrelRef` (`self.TankBarrel`))
  (`self.SetTurretRef` (`self.TankTurret`)))

(event `InputAxis|AimX`
  (params (AxisValue :type "Float (single-precision)"))
  (`SceneComponent.K2_AddLocalRotation` (`self.Gimbal`) (`KismetMathLibrary.MakeRotator` 0.0 0.0 AxisValue) false false))

(event `InputAxis|AimY`
  (params (AxisValue :type "Float (single-precision)"))
  (`SceneComponent.K2_AddLocalRotation` (`self.SpringArm`) (`KismetMathLibrary.MakeRotator` 0.0 AxisValue) false false))

(event `InputAction|Fire`
  (params (Key :type "Key Structure"))
  (:`Pressed`
    (`self.fire`)))

(fn `UserConstructionScript`)